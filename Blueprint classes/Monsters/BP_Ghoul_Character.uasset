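; Ghoul monster character that reacts to hits, plays its sounds and detects the player in melee range.
; BeginPlay binds damage and sound delegates; the sound delegate spawns the ghoul cue attached to the mesh.
; Damage briefly activates a particle effect at the hit bone and spawns a temporary blood decal near the Cube component with random Y offset.
; Player overlap with AttackBox sets a flag and triggers the attack call to the AI controller.
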(event `self.ReceiveBeginPlay`
  (add `self.OnTakingDamage` (delegate `OnTakingDamage_Event_0`))
  (add `self.OnplaySound_Del` (delegate `OnplaySound_Del_Event_0`)))

(event `OnTakingDamage_Event_0` :!signature `self.OnTakingDamage`
  (params (BoneName :type Name))
  (`self.Took Damage` BoneName))

(event `OnplaySound_Del_Event_0`
  (`GameplayStatics.SpawnSoundAttached` "/Game/MAEOakForest/Sounds/Monster_Sounds/Ghoul_Sounds/GhoulSoundsCue.GhoulSoundsCue" (`self.Mesh`) "Head" (0.0 0.0 0.0) (struct) "KeepRelativeOffset" false 1.0 1.2 0.0 null null))

(event `self.Attack Box.OnComponentBeginOverlap`
  (params (OverlappedComponent :type "PrimitiveComponent Object Reference") (OtherActor :type "Actor Object Reference") (OtherComp :type "PrimitiveComponent Object Reference") (OtherBodyIndex :type Integer) (bFromSweep :type Boolean) (SweepResult :type "HitResult Structure (by ref)"))
  (if (== (`GameplayStatics.GetPlayerPawn` 0) OtherActor)
    (set `self.OverlappedAttackBox` true)
    (`self.CallAttack_InAICon`)))

(event `Took Damage`
  (params (`Bone Name` :type Name))
  (bind _particlesystem (`self.ParticleSystem`))
  (bind (_returnvalue_x _returnvalue_y _returnvalue_z) (`KismetMathLibrary.BreakVector` (`SceneComponent.K2_GetComponentLocation` (`self.Cube`))))
  (`ActorComponent.Activate` _particlesystem false)
  (`SceneComponent.K2_SetWorldLocation` _particlesystem (`SceneComponent.GetSocketLocation` (`self.Mesh`) `Bone Name`) false false)
  (`GameplayStatics.SpawnDecalAtLocation` "/Game/Megascans/Decals/High_Velocity_Blood_Spatter_sfijfbip/MI_High_Velocity_Blood_Spatter_sfijfbip_4K.MI_High_Velocity_Blood_Spatter_sfijfbip_4K" (3.0 70.0 70.0) (`KismetMathLibrary.MakeVector` _returnvalue_x (+ _returnvalue_y (`KismetMathLibrary.RandomFloatInRange` -70.0 70.0)) _returnvalue_z) (struct :`Pitch` -90.0) 120.0)
  (`KismetSystemLibrary.Delay` 0.5)
  (`ActorComponent.Deactivate` (`self.ParticleSystem`)))

(fn `UserConstructionScript`)