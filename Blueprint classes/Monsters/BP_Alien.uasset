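; Alien monster character that reacts to attack and dodge broadcasts with motion-warped melee attacks and dodge target selection.
; On attack, it stops movement, warps toward player 0's current location (ignoring the broadcast location) and plays the flip kick, backhand or kick montage by attack number.
; On dodge, it only stores a destination: offset from the player in world X, or randomly right, left or back, as the forward case is unreachable.
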(event `self.ReceiveBeginPlay`
  (add `self.OnAttackingCast` (delegate `OnAttackingCast_Event_0`))
  (add `self.OnDodge` (delegate `OnDodge_Event_0`)))

(event `OnDodge_Event_0`
  (`self.On Dodge Set Main Dodge Location`))

(event `OnAttackingCast_Event_0` :!signature `self.OnAttackingCast`
  (params (AttackNumber :type Integer) (AttackLocation :type "Vector Structure"))
  (`self.Warp On Attacking ` AttackNumber AttackLocation)
  (`KismetSystemLibrary.PrintString` "Broad Cast is Working " true true (struct :`R` 0.660203 :`B` 1.0 :`A` 1.0) 6.0))

(event `On Dodge Set Main Dodge Location`
  (bind (_returnvalue_x _returnvalue_y _returnvalue_z) (`KismetMathLibrary.BreakVector` (`self.K2_GetActorLocation`)))
  (bind (_returnvalue_x_2 _returnvalue_y_2) (`KismetMathLibrary.BreakVector` (`self.K2_GetActorLocation` (`GameplayStatics.GetPlayerPawn` 0))))
  (if (`self.DodgeToPlayer`)
    (set `self.MainDodgeLocation` (`KismetMathLibrary.MakeVector` (+ _returnvalue_x_2 400.0) _returnvalue_y_2 _returnvalue_z))
    (else
      (switch `int` (`KismetMathLibrary.RandomInteger` 3)
        (:`0`
          (set `self.MainDodgeLocation` (`SceneComponent.K2_GetComponentLocation` (`self.Right Location`))))
        (:`1`
          (set `self.MainDodgeLocation` (`SceneComponent.K2_GetComponentLocation` (`self.Left Location`))))
        (:`2`
          (set `self.MainDodgeLocation` (`SceneComponent.K2_GetComponentLocation` (`self.Back Location`))))
        (:`3`
          (set `self.MainDodgeLocation` (`SceneComponent.K2_GetComponentLocation` (`self.Forward Location`))))))))

(fn `UserConstructionScript`)

(fn `Warp On Attacking `
  (params (`Attack Number` :type Integer) (`Player Location ` :type "Vector Structure"))
  (bind _returnvalue (`self.K2_GetActorLocation` (`GameplayStatics.GetPlayerPawn` 0)))
  (switch `int` `Attack Number`
    (:`0`
      (`MovementComponent.StopMovementImmediately` (`self.CharacterMovement`))
      (`MotionWarpingComponent.AddOrUpdateWarpTargetFromTransform` (`self.MotionWarping`) "Flip Kick" (`KismetMathLibrary.Conv_VectorToTransform` _returnvalue))
      (`self.PlayAnimMontage` "/Game/Characters_Meshs/Hybrid_Monster/Animations/Attacking/Attacks_Test/KickRotate_AttackMon_Hybrid.KickRotate_AttackMon_Hybrid"))
    (:`1`
      (`MovementComponent.StopMovementImmediately` (`self.CharacterMovement`))
      (`MotionWarpingComponent.AddOrUpdateWarpTargetFromTransform` (`self.MotionWarping`) "Hand Attack" (`KismetMathLibrary.Conv_VectorToTransform` _returnvalue))
      (`self.PlayAnimMontage` "/Game/Characters_Meshs/Hybrid_Monster/Animations/Attacking/Another_AttackAnim/Standing_Melee_Attack_Backhand_Montage.Standing_Melee_Attack_Backhand_Montage")
      (`KismetSystemLibrary.PrintString` "Warp Second Attack" true true (struct :`R` 1.0 :`G` 0.965634 :`A` 1.0) 6.0))
    (:`2`
      (`MovementComponent.StopMovementImmediately` (`self.CharacterMovement`))
      (`MotionWarpingComponent.AddOrUpdateWarpTargetFromTransform` (`self.MotionWarping`) "Kick" (`KismetMathLibrary.Conv_VectorToTransform` _returnvalue))
      (`self.PlayAnimMontage` "/Game/Characters_Meshs/Hybrid_Monster/Animations/Attacking/Attacks_Test/LeftKick_AttackMon_Hybrid.LeftKick_AttackMon_Hybrid"))))