(event `self.ReceiveBeginPlay`
  (bind _returnvalue (`GameUserSettings.GetGameUserSettings`))
  (`GameUserSettings.SetVSyncEnabled` _returnvalue true)
  (bind _ascpp_game_ins_tance (cast `CPP_Game_Ins_tance` (`GameplayStatics.GetGameInstance`)))
  (set `self.As CPP Game Ins Tance` _ascpp_game_ins_tance)
  (add `self.OnPlayerDeath` (delegate `OnPlayerDeath_Event_1`))
  (bind _returnvalue_2 (`|CreateWidget` "/Game/MyBlueprints/Widgets/Player_UI_Widgets/Health_And_Hunger_Widget.Health_And_Hunger_Widget_C"))
  (bind _output_get (set `self.Health_And_Hunger_WidgetRef` _returnvalue_2))
  (`self.On Health Update`)
  (`UserWidget.AddToViewport` _output_get 0)
  (`self.On Player Taking Damage`)
  (`self.On Hunger Change `)
  (add `self.OnTakingDamage_Del` (delegate `OnTakingDamage_Del_Event_1`))
  (add `self.OnHealth_Update_Del` (delegate `OnHealth_Update_Del_Event_1`))
  (add `self.OnHungerChange_Del` (delegate `OnHungerChange_Del_Event_1`))
  (`KismetSystemLibrary.Delay` 500.0)
  (`self.Instruction Press (I)`))

(event `OnPlayerDeath_Event_1`
  (`self.On Player Death1`))

(event `OnTakingDamage_Del_Event_1`
  (`self.On Player Taking Damage`))

(event `OnHungerChange_Del_Event_1`
  (`self.On Hunger Change `))

(event `OnHealth_Update_Del_Event_1`
  (`self.On Health Update`))

(event `self.ReceiveTick`
  (params (DeltaSeconds :type "Float (single-precision)"))
  (`self.Camera Shake Head Bop`))

(event `On Player Taking Damage`
  (if (`self.Already Created Blood Splatter Widget`)
    (`/Game/MyBlueprints/Widgets/Player_UI_Widgets/Blood_Splatter_Widget.Play_GotHitAnimation` (`self.Blood Splatter Widget Referance`))
    ;[1 1 1] Instruction for players
    (`/Engine/EditorBlueprintResources/StandardMacros.DoOnce` false
      (:`Completed`
        (bind _returnvalue (`|CreateWidget` "/Game/MyBlueprints/Widgets/Player_UI_Widgets/instructions_Widget.instructions_Widget_C"))
        (`UserWidget.AddToViewport` _returnvalue 0)
        (bind _foundwidgets (`WidgetBlueprintLibrary.GetAllWidgetsOfClass` "/Game/MyBlueprints/Widgets/Player_UI_Widgets/instructions_Widget.instructions_Widget_C"))
        (message `/Game/MyBlueprints/Widgets/Player_UI_Widgets/Player_Widgets_Interface.Update instructions Text` _returnvalue "You restore health when your hunger is above 90%" (`KismetMathLibrary.Conv_IntToInt64` (`KismetArrayLibrary.Array_Length` _foundwidgets)))
        (`KismetSystemLibrary.Delay` 10.0)
        (`Widget.RemoveFromParent` _returnvalue)))
    (else
      (bind _returnvalue_2 (`|CreateWidget` "/Game/MyBlueprints/Widgets/Player_UI_Widgets/Blood_Splatter_Widget.Blood_Splatter_Widget_C"))
      (bind _output_get (set `self.Blood Splatter Widget Referance` _returnvalue_2))
      (`UserWidget.AddToViewport` _output_get 0)
      (set `self.Already Created Blood Splatter Widget` true))))

(event `On Hunger Change`
  (message `/Game/MyBlueprints/Widgets/Player_UI_Widgets/Player_Widgets_Interface.Update Health And Hunger ` (`self.Health_And_Hunger_WidgetRef`) (`self.PlayerHealth`) (`self.InitialHealth`) (`self.Hunger`)))

(event `Key|I`
  (params (Key :type "Key Structure"))
  (bind _returnvalue (`GameplayStatics.GetPlayerController` 0))
  (bind _returnvalue_2 (`GameplayStatics.GetPlayerController` 0))
  ;[1 1 1] Inventory Input
  (:`Pressed`
    (if (`self.Is Inventory Widget OS`)
      (`Widget.RemoveFromParent` (`self.Inventory Widget Ref`))
      (set `self.Is Inventory Widget OS` false)
      (`WidgetBlueprintLibrary.SetInputMode_GameOnly` _returnvalue_2)
      (set `PlayerController.bShowMouseCursor` false _returnvalue_2)
      (else
        (bind _returnvalue_3 (`|CreateWidget` "/Game/MyBlueprints/Widgets/Inventory_Widgets/Inventory_MainWidget.Inventory_MainWidget_C"))
        (set `self.Inventory Widget Ref` _returnvalue_3)
        (`UserWidget.AddToViewport` _returnvalue_3 0)
        (set `self.Is Inventory Widget OS` true)
        (`WidgetBlueprintLibrary.SetInputMode_GameAndUIEx` _returnvalue null)
        (set `PlayerController.bShowMouseCursor` true _returnvalue)))))

(event `On Health Update`
  (message `/Game/MyBlueprints/Widgets/Player_UI_Widgets/Player_Widgets_Interface.Update Health And Hunger ` (`self.Health_And_Hunger_WidgetRef`) (`self.PlayerHealth`) (`self.InitialHealth`) (`self.Hunger`)))

(event `Key|J`
  (params (Key :type "Key Structure"))
  (bind _returnvalue (`GameplayStatics.GetPlayerController` 0))
  ;[1 1 1] Diary Input
  (:`Pressed`
    (if (`self.HasDiary`)
      (if (`self.In Diary Widget OS`)
        (`Widget.RemoveFromParent` (`self.Book Widget`))
        (set `PlayerController.bShowMouseCursor` false _returnvalue)
        (`WidgetBlueprintLibrary.SetInputMode_GameOnly` _returnvalue)
        (set `self.In Diary Widget OS` false)
        (else
          (bind _returnvalue_2 (`|CreateWidget` "/Game/MyBlueprints/Widgets/Diary_Widgets/Diary_First_Page.Diary_First_Page_C"))
          (bind _output_get (set `self.Book Widget` _returnvalue_2))
          (`UserWidget.AddToViewport` _output_get 0)
          (set `self.In Diary Widget OS` true))))))

(event `Camera Shake Head Bop`
  (bind _returnvalue (`GameplayStatics.GetPlayerController` 0))
  (bind _returnvalue_2 (`KismetMathLibrary.VSize` (`self.GetVelocity`)))
  (if (<= _returnvalue_2 0.0)
    (`PlayerController.ClientStartCameraShake` :`self` _returnvalue :`Shake` "/Game/MyBlueprints/Camera_Shake/Idle_Shake.Idle_Shake_C")
    (elif (<= _returnvalue_2 350.0)
      (`PlayerController.ClientStartCameraShake` :`self` _returnvalue :`Shake` "/Game/MyBlueprints/Camera_Shake/Walk_Shake.Walk_Shake_C")
      (else
        (`PlayerController.ClientStartCameraShake` :`self` _returnvalue :`Shake` "/Game/MyBlueprints/Camera_Shake/Sprinting_Shake.Sprinting_Shake_C")))))

(event `Key|Escape`
  (params (Key :type "Key Structure"))
  (bind _returnvalue (`GameplayStatics.GetPlayerController` 0))
  (bind _returnvalue_2 (`GameplayStatics.GetPlayerController` 0))
  (bind _inventory_widget_ref (`self.Inventory Widget Ref`))
  (bind _book_widget (`self.Book Widget`))
  ;[1 1 1] Pause Input
  (:`Pressed`
    (bind _returnvalue_3 (`|CreateWidget` "/Game/MyBlueprints/Widgets/Pause_Menu_Wdgets/Pause_Menu_Widget.Pause_Menu_Widget_C"))
    (if (`Widget.IsInViewport` _returnvalue_3)
      (`Widget.RemoveFromParent` _returnvalue_3)
      (elif (`Widget.IsInViewport` _inventory_widget_ref)
        (`Widget.RemoveFromParent` _inventory_widget_ref)
        (set `PlayerController.bShowMouseCursor` false _returnvalue_2)
        (`WidgetBlueprintLibrary.SetInputMode_GameOnly` _returnvalue_2)
        (set `self.Is Inventory Widget OS` false)
        (else
          (`/Engine/EditorBlueprintResources/StandardMacros.IsValid` _book_widget
            (:`Is Valid`
              (if (`Widget.IsInViewport` _book_widget)
                (`Widget.RemoveFromParent` _book_widget)
                (set `PlayerController.bShowMouseCursor` false _returnvalue)
                (`WidgetBlueprintLibrary.SetInputMode_GameOnly` _returnvalue)
                (set `self.In Diary Widget OS` false)
                (else
                  (`UserWidget.AddToViewport` _returnvalue_3 0 :!label _label))))
            (:`Is Not Valid`
              (goto _label))))))))

(fn `Instruction Press (I)`
  (`KismetSystemLibrary.PrintString` "Added on the screen  I " true true (struct :`R` 0.945618 :`G` 1.0 :`A` 1.0) 4.0)
  (bind _returnvalue (`|CreateWidget` "/Game/MyBlueprints/Widgets/Player_UI_Widgets/instructions_Widget.instructions_Widget_C"))
  (`UserWidget.AddToViewport` _returnvalue 0)
  (bind _foundwidgets (`WidgetBlueprintLibrary.GetAllWidgetsOfClass` "/Game/MyBlueprints/Widgets/Player_UI_Widgets/instructions_Widget.instructions_Widget_C"))
  (message `/Game/MyBlueprints/Widgets/Player_UI_Widgets/Player_Widgets_Interface.Update instructions Text` _returnvalue "[ i ] Open and close inventory" (`KismetMathLibrary.Conv_IntToInt64` (`KismetArrayLibrary.Array_Length` _foundwidgets))))

(fn `On Player Death1`
  (bind _returnvalue (`GameplayStatics.GetPlayerController` 0))
  (bind _returnvalue_2 (`|CreateWidget` "/Game/MyBlueprints/Widgets/PlayerDeadWidget.PlayerDeadWidget_C"))
  (`self.PlayAnimMontage` "/Game/Characters_Meshs/Player_SkeletonMesh/Animations/Standing_Death_Backward_01__1__Montage.Standing_Death_Backward_01__1__Montage")
  (`UserWidget.AddToViewport` _returnvalue_2 0)
  (set `PlayerController.CurrentMouseCursor` "Hand" _returnvalue)
  (set `PlayerController.bShowMouseCursor` true _returnvalue))

(fn `Return Player Inventroy Ref`
  (returns (`Inventory Ref` :type "Inventory_System_AC Object Reference") (`player Ref` :type "/Blueprint classes/Player_Blueprint/BP_Survivor_Character Object Reference"))
  (return (`self.Inventory_System_AC`) self))

(fn `UserConstructionScript`)