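; BP_IBA_Log is a log item that shows an instruction, noted as how to drop with G, when picked up as an unstorable item.
; BeginPlay caches the game instance and binds the pickup delegate, whose handler runs once.
; The handler skips text already in the game instance's InstructionsTexts list.
; Otherwise it creates an Instructions_Widget, passes it the text and on-screen widget count, and records the text.
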(event `self.ReceiveBeginPlay`
  (bind _ascpp_game_ins_tance (cast `CPP_Game_Ins_tance` (`GameplayStatics.GetGameInstance`)))
  (set `self.As CPP Game Ins Tance` _ascpp_game_ins_tance)
  (add `self.OnPickingUp_UnstorableItem_Del` (delegate `OnPickingUp_UnstorableItem_Del_Event_0`)))

(event `OnPickingUp_UnstorableItem_Del_Event_0`
  ;[1 1 1] Drop With G Instruction
  (`/Engine/EditorBlueprintResources/StandardMacros.DoOnce` false
    (:`Completed`
      (for _array_element (`CPP_Game_Ins_tance.Instructions_texts` (`self.As CPP Game Ins Tance`))
        (if (`KismetTextLibrary.EqualEqual_TextText` _array_element (`KismetTextLibrary.Conv_StringToText` (`self.Text`)))
          (set `self.Text_AlreadyShowed` true)))
      (if (not (`self.Text_AlreadyShowed`))
        (bind _returnvalue (`|CreateWidget` "/Game/MyBlueprints/Widgets/Player_UI_Widgets/instructions_Widget.instructions_Widget_C"))
        (`UserWidget.AddToViewport` _returnvalue 0)
        (bind _foundwidgets (`WidgetBlueprintLibrary.GetAllWidgetsOfClass` "/Game/MyBlueprints/Widgets/Player_UI_Widgets/instructions_Widget.instructions_Widget_C"))
        (message `/Game/MyBlueprints/Widgets/Player_UI_Widgets/Player_Widgets_Interface.Update instructions Text` _returnvalue (`self.Text`) (`KismetMathLibrary.Conv_IntToInt64` (`KismetArrayLibrary.Array_Length` _foundwidgets)))
        (`KismetArrayLibrary.Array_Add` (`CPP_Game_Ins_tance.Instructions_texts` (`self.As CPP Game Ins Tance`)) (`KismetTextLibrary.Conv_StringToText` (`self.Text`)))))))

(fn `UserConstructionScript`)